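; Pickup actor that unlocks the Dash ability by setting DashLearned on the Puzzle Island game instance.
; On BeginPlay it caches the game instance and destroys itself if Dash is already learned.
; Any overlap with its collision sphere, with no check on the overlapping actor, sets the flag and shows an Info_Text_Important message.
; The actor then hides, waits briefly, removes the widget and destroys itself.
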(event OnComponentBeginOverlap(CollisionSphere)
  (params (OverlappedComponent :type Primitive%20Component%20Object%20Reference) (OtherActor :type Actor%20Object%20Reference) (OtherComp :type Primitive%20Component%20Object%20Reference) (OtherBodyIndex :type Integer) (bFromSweep :type Boolean) (SweepResult :type Hit%20Result%20Structure%20%28by%20ref%29))
  (Variables|/Game/Blueprints/Puzzle_Island_Instance_BP.Puzzle_Island_Instance_BP_C|SetDashLearned (Variables|Default|GetGameInstance) true)
  (bind _returnvalue (UserInterface|CreateWidget "/Game/Blueprints/Info_Text_Important.Info_Text_Important_C" (Game|GetPlayerController 0) "You have learned Dash. Press Left Shift to use."))
  (bind _output_get (Variables|Default|SetLearned_Dash_Text_Wid _returnvalue))
  (UserInterface|Viewport|AddtoViewport _output_get 0)
  (Rendering|SetActorHiddenInGame self true)
  (Utilities|FlowControl|Delay 2.0)
  (Widget|RemovefromParent (Variables|Default|GetLearned_Dash_Text_Wid))
  (Actor|DestroyActor))

(event EventBeginPlay
  (bind _aspuzzle_island_instance_bp (Utilities|Casting|CastToPuzzle_Island_Instance_BP (Game|GetGameInstance)))
  (Variables|Default|SetGameInstance _aspuzzle_island_instance_bp)
  (if (Variables|/Game/Blueprints/Puzzle_Island_Instance_BP.Puzzle_Island_Instance_BP_C|GetDashLearned _aspuzzle_island_instance_bp)
    (Actor|DestroyActor)))

(event Collision|EventActorBeginOverlap
  (params (OtherActor :type Actor%20Object%20Reference)))

(event EventTick
  (params (DeltaSeconds :type Float%20%28single-precision%29)))

(fn ConstructionScript)