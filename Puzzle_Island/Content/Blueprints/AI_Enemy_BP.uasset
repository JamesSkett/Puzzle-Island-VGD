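; AI_Enemy_BP is an enemy that wanders the navmesh until it sees the player, then chases them.
; While not InRange, Tick starts a move to a random navigable point within a radius, using a Moving flag to avoid reissuing it until success or failure.
; PawnSensing's OnSeePawn sets InRange and starts an AI move toward any seen ThirdPersonCharacter; nothing clears InRange, so wandering never resumes.
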(event OnSeePawn(PawnSensing)
  (params (Pawn :type Pawn%20Object%20Reference))
  (Variables|Default|SetIn_Range true)
  (bind _asthird_person_character (Utilities|Casting|CastToThirdPersonCharacter Pawn))
  (AI|AIMoveTo self "0, 0, 0" _asthird_person_character 5.0 false))

(event EventBeginPlay)

(event Collision|EventActorBeginOverlap
  (params (OtherActor :type Actor%20Object%20Reference)))

(event EventTick
  (params (DeltaSeconds :type Float%20%28single-precision%29))
  (if (not (Variables|Default|GetIn_Range))
    (if (not (Variables|Default|GetMoving))
      (AI|AIMoveTo self (.RandomLocation (Class|NavigationSystem|GetRandomPointinNavigableRadius (Transformation|GetActorLocation) 5e+02)) 0 5.0 false
        (:then
          (Variables|Default|SetMoving true))
        (:OnSuccess
          (Variables|Default|SetMoving false :!label _label))
        (:OnFail
          (goto _label))))))

(fn ConstructionScript)