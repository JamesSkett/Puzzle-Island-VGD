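; Game instance Blueprint for a puzzle island game, holding player progress and providing a function to reset it.
; ResetGame clears completion and star counts for the jigsaw puzzles, jump puzzle completion, the door unlock and the total star count.
; It also clears dash and sprint ability state along with related UI flags, and restores the saved character location to a fixed starting point.
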(fn ResetGame
  (Variables|JigsawPuzzleVar|SetJigsaw_01_Complete false)
  (Variables|JigsawPuzzleVar|SetJigsaw_01_StarsEarned 0)
  (Variables|JigsawPuzzleVar|SetJigsaw_02_Complete false)
  (Variables|JigsawPuzzleVar|SetJigsaw_02_StarsEarned 0)
  (Variables|JigsawPuzzleVar|SetJigsaw_03_Complete false)
  (Variables|JigsawPuzzleVar|SetJigsaw_03_StarsEarned 0)
  (Variables|PlayerVar|SetCharacterLocation "-8116.000000,12538.000000,677.000000")
  (Variables|PlayerVar|SetStarsCount 0)
  (Variables|PlayerAbilities|SetDashLearned false)
  (Variables|PlayerAbilities|SetSprintLearned false)
  (Variables|PlayerAbilities|SetDashLearnedTextOnce false)
  (Variables|PlayerAbilities|SetSprintImageSet false)
  (Variables|PlayerAbilities|SetAbility01_Sprint_Learned false)
  (Variables|PlayerAbilities|SetAbility01_Selected false)
  (Variables|Doors|SetDoor_01_Unlocked false)
  (Variables|JumpingPuzzleNpcVar|SetJump_Puzzle01Complete false)
  (Variables|JumpingPuzzleNpcVar|SetJump_Puzzle02_Complete false))