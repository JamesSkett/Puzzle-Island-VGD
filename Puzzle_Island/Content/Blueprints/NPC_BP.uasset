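; NPC actor that shows a text box when the player is nearby and then sends them into a level, likely a puzzle.
; A trigger overlap tracks whether the player is near, and leaving it closes the text box.
; Pressing E nearby creates the NPC_TextBox widget with the NPC's text.
; Pressing E again closes it, sets IsLoading on ThirdPersonCharacter, and opens LevelName after a short delay.
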(event OnComponentBeginOverlap(Trigger)
  (params (OverlappedComponent :type Primitive%20Component%20Object%20Reference) (OtherActor :type Actor%20Object%20Reference) (OtherComp :type Primitive%20Component%20Object%20Reference) (OtherBodyIndex :type Integer) (bFromSweep :type Boolean) (SweepResult :type Hit%20Result%20Structure%20%28by%20ref%29))
  ;[1 1 1] Load into the puzzle
  (Variables|Default|SetIs_Near_NPC true))

(event OnComponentEndOverlap(Trigger)
  (params (OverlappedComponent :type Primitive%20Component%20Object%20Reference) (OtherActor :type Actor%20Object%20Reference) (OtherComp :type Primitive%20Component%20Object%20Reference) (OtherBodyIndex :type Integer))
  ;[1 1 1] Load into the puzzle
  (Variables|Default|SetIs_Near_NPC false)
  (if (Variables|Default|GetText_Widget_Is_Displayed)
    (Widget|RemovefromParent (stale Input|KeyboardEvents|E _returnvalue))
    (Variables|Default|SetText_Widget_Is_Displayed false)))

(event Collision|EventActorBeginOverlap
  (params (OtherActor :type Actor%20Object%20Reference)))

(event EventTick
  (params (DeltaSeconds :type Float%20%28single-precision%29)))

(event Input|KeyboardEvents|E
  (params (Key :type Key%20Structure))
  ;[1 1 1] Load into the puzzle
  (:Pressed
    (if (Variables|Default|GetText_Widget_Is_Displayed)
      (Widget|RemovefromParent (stale _returnvalue))
      (Variables|Default|SetText_Widget_Is_Displayed false)
      (bind _asthird_person_character (Utilities|Casting|CastToThirdPersonCharacter (Game|GetPlayerCharacter 0)))
      (Variables|/Game/Blueprints/ThirdPersonCharacter.ThirdPersonCharacter_C|SetIsLoading _asthird_person_character true)
      (Utilities|FlowControl|Delay 2.0)
      (Game|OpenLevel(byName) (Variables|Default|GetLevel_Name))
      (elif (Variables|Default|GetIs_Near_NPC)
        (bind _returnvalue (UserInterface|CreateWidget "/Game/Blueprints/NPC_TextBox.NPC_TextBox_C" (Game|GetPlayerController 0)))
        (Default|UpdateText _returnvalue (Variables|Default|GetNPC_Text_To_Display))
        (UserInterface|Viewport|AddtoViewport _returnvalue 0)
        (Variables|Default|SetText_Widget_Is_Displayed true)))))

(fn ConstructionScript)