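; Jigsaw puzzle piece Blueprint that shows an assigned sprite and can be dragged with the mouse.
; On BeginPlay it applies the sprite and enables click events on the player controller.
; Sprite click and release events toggle a flag, and while it is set, Tick moves the sprite component to the deprojected mouse world position.
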(event OnClicked(PieceSprite)
  (params (TouchedComponent :type Primitive%20Component%20Object%20Reference) (ButtonPressed :type Key%20Structure))
  (Variables|Default|SetIsClicked true))

(event OnReleased(PieceSprite)
  (params (TouchedComponent :type Primitive%20Component%20Object%20Reference) (ButtonReleased :type Key%20Structure))
  (Variables|Default|SetIsClicked false))

(event EventBeginPlay
  (Rendering|Components|Sprite|SetSprite (Variables|Default|GetPieceSprite) (Variables|Default|GetSprite))
  (Variables|/Script/Engine.PlayerController|SetbEnableClickEvents (Game|GetPlayerController 0) true))

(event EventTick
  (params (DeltaSeconds :type Float%20%28single-precision%29))
  (if (Variables|Default|GetIsClicked)
    (Transformation|SetWorldLocation (Variables|Default|GetPieceSprite) (.WorldLocation (Game|Player|ConvertMouseLocationToWorldSpace (Game|GetPlayerController 0))) false false)))

(fn ConstructionScript)