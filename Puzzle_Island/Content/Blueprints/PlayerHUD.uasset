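; PlayerHUD is a HUD Blueprint that shows a full-screen loading overlay during play.
; Each DrawHUD pass casts the player character to ThirdPersonCharacter and reads its IsLoading flag.
; While that flag is set, it draws the LoadingScreen_Mat material across the whole screen using the canvas size.
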(event EventBeginPlay)

(event Collision|EventActorBeginOverlap
  (params (OtherActor :type Actor%20Object%20Reference)))

(event EventTick
  (params (DeltaSeconds :type Float%20%28single-precision%29)))

(event EventDrawHUD
  (params (SizeX :type Integer) (SizeY :type Integer))
  (Variables|Default|SetScreenDimentions (Math|Vector2D|MakeVector2D (Math|Conversions|ToFloat(Integer) SizeX) (Math|Conversions|ToFloat(Integer) SizeY)))
  (bind _asthird_person_character (Utilities|Casting|CastToThirdPersonCharacter (Game|GetPlayerCharacter 0)))
  (if (Variables|/Game/Blueprints/ThirdPersonCharacter.ThirdPersonCharacter_C|GetIsLoading _asthird_person_character)
    (Class|HUD|DrawMaterialSimple "/Game/Materials/LoadingScreen_Mat.LoadingScreen_Mat" 0.0 0.0 (.X (Math|Vector2D|BreakVector2D (Variables|Default|GetScreenDimentions))) (.Y (Math|Vector2D|BreakVector2D (Variables|Default|GetScreenDimentions))) 1.0 false)))

(fn ConstructionScript)