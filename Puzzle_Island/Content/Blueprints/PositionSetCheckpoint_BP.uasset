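; Checkpoint actor that records the player's position when the ThirdPersonCharacter overlaps its TriggerBox.
; On each overlap it writes the character's location into CharacterLocation on the Puzzle_Island_Instance_BP game instance.
; If NotifyChecpointReached is set, the first overlap also shows an Info_Text "Checkpoint Reached." widget for two seconds, guarded by the CheckpointReached flag.
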(event OnComponentBeginOverlap(TriggerBox)
  (params (OverlappedComponent :type Primitive%20Component%20Object%20Reference) (OtherActor :type Actor%20Object%20Reference) (OtherComp :type Primitive%20Component%20Object%20Reference) (OtherBodyIndex :type Integer) (bFromSweep :type Boolean) (SweepResult :type Hit%20Result%20Structure%20%28by%20ref%29))
  (bind _asthird_person_character (Utilities|Casting|CastToThirdPersonCharacter OtherActor))
  (Variables|/Game/Blueprints/Puzzle_Island_Instance_BP.Puzzle_Island_Instance_BP_C|SetCharacterLocation (.AsPuzzle%20Island%20Instance%20BP (Utilities|Casting|CastToPuzzle_Island_Instance_BP (Game|GetGameInstance))) (Transformation|GetActorLocation _asthird_person_character))
  (if (Variables|Default|GetNotifyChecpointReached)
    (if (not (Variables|Default|GetCheckpointReached))
      (Variables|Default|SetCheckpointReached true)
      (bind _returnvalue (UserInterface|CreateWidget "/Game/Blueprints/Info_Text.Info_Text_C" (Game|GetPlayerController 0) "Checkpoint Reached."))
      (UserInterface|Viewport|AddtoViewport _returnvalue 0)
      (Utilities|FlowControl|Delay 2.0)
      (Widget|RemovefromParent _returnvalue))))

(event EventBeginPlay)

(event Collision|EventActorBeginOverlap
  (params (OtherActor :type Actor%20Object%20Reference)))

(event EventTick
  (params (DeltaSeconds :type Float%20%28single-precision%29)))

(fn ConstructionScript)