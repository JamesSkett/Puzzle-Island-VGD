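; Interactive NPC at the end of the second jumping puzzle that rewards the player and offers a teleport to safety.
; Pressing E inside its trigger shows a text box, granting stars once and recording completion in the game instance.
; Further presses show the teleport offer, then move the player to a fixed location and flag a sprint hat pickup to spawn.
; Leaving the trigger dismisses the text box.
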(event OnComponentBeginOverlap(Trigger)
  (params (OverlappedComponent :type Primitive%20Component%20Object%20Reference) (OtherActor :type Actor%20Object%20Reference) (OtherComp :type Primitive%20Component%20Object%20Reference) (OtherBodyIndex :type Integer) (bFromSweep :type Boolean) (SweepResult :type Hit%20Result%20Structure%20%28by%20ref%29))
  (Variables|Default|SetIs_Near_NPC true))

(event OnComponentEndOverlap(Trigger)
  (params (OverlappedComponent :type Primitive%20Component%20Object%20Reference) (OtherActor :type Actor%20Object%20Reference) (OtherComp :type Primitive%20Component%20Object%20Reference) (OtherBodyIndex :type Integer))
  (Variables|Default|SetIs_Near_NPC false)
  (if (Variables|Default|GetText_Widget_Is_Displayed)
    (Widget|RemovefromParent (Variables|Default|GetTextWidget))
    (Variables|Default|SetText_Widget_Is_Displayed false)
    (Variables|Default|SetTeleportMessageDisplayed false)))

(event EventBeginPlay
  (bind _aspuzzle_island_instance_bp (Utilities|Casting|CastToPuzzle_Island_Instance_BP (Game|GetGameInstance)))
  (Variables|Default|SetGameInstance _aspuzzle_island_instance_bp))

(event Input|KeyboardEvents|E
  (params (Key :type Key%20Structure))
  (bind _gameinstance (Variables|Default|GetGameInstance))
  ;[1 1 1] NPC textbox create, award stars
  (:Pressed
    (if (Variables|Default|GetIs_Near_NPC)
      (if (Variables|Default|GetTeleportMessageDisplayed)
        (Variables|/Game/Blueprints/Puzzle_Island_Instance_BP.Puzzle_Island_Instance_BP_C|SetSpawnSprintPickup (Variables|Default|GetGameInstance) true)
        (Transformation|SetActorLocation (Game|GetPlayerCharacter 0) "-2265.000000,-3314.000000,742.703308" false false)
        (if (Utilities|IsValid (Variables|Default|GetTextWidget))
          (Widget|RemovefromParent (Variables|Default|GetTextWidget))
          (Variables|Default|SetText_Widget_Is_Displayed false)
          (Variables|Default|SetTeleportMessageDisplayed false)
          (Variables|Default|SetIs_Near_NPC false))
        (elif (Variables|/Game/Blueprints/Puzzle_Island_Instance_BP.Puzzle_Island_Instance_BP_C|GetJump_Puzzle02_Complete (Variables|Default|GetGameInstance))
          (if (Variables|Default|GetText_Widget_Is_Displayed)
            (Default|UpdateText (Variables|Default|GetTextWidget) "Let me teleport  you to safety." :!label _label)
            (Variables|Default|SetTeleportMessageDisplayed true)
            (else
              (bind _returnvalue (UserInterface|CreateWidget "/Game/Blueprints/NPC_TextBox.NPC_TextBox_C" (Game|GetPlayerController 0)))
              (Variables|Default|SetTextWidget _returnvalue)
              (Default|UpdateText _returnvalue "You have already received reward for this jumping puzzle.")
              (UserInterface|Viewport|AddtoViewport _returnvalue 0)
              (Variables|Default|SetText_Widget_Is_Displayed true)))
          (elif (Variables|Default|GetText_Widget_Is_Displayed)
            (goto _label)
            (elif (Variables|Default|GetIs_Near_NPC)
              (bind _returnvalue_2 (UserInterface|CreateWidget "/Game/Blueprints/NPC_TextBox.NPC_TextBox_C" (Game|GetPlayerController 0)))
              (Variables|Default|SetTextWidget _returnvalue_2)
              (Default|UpdateText _returnvalue_2 (Utilities|Text|ToText(String) (Utilities|String|Append "Well done. I will reward you with " (Utilities|String|ToString(Integer) (Variables|Default|GetStarsRewardAmount)) " stars for completing this puzzle and a new leopard hat that will alow you to explore the island faster. Use it with right mouse button. Pick it up!!!")))
              (UserInterface|Viewport|AddtoViewport _returnvalue_2 0)
              (Variables|Default|SetText_Widget_Is_Displayed true)
              (Variables|/Game/Blueprints/Puzzle_Island_Instance_BP.Puzzle_Island_Instance_BP_C|SetJump_Puzzle02_Complete _gameinstance true)
              (Variables|/Game/Blueprints/Puzzle_Island_Instance_BP.Puzzle_Island_Instance_BP_C|SetStarsCount _gameinstance (+ (Variables|/Game/Blueprints/Puzzle_Island_Instance_BP.Puzzle_Island_Instance_BP_C|GetStarsCount _gameinstance) (Variables|Default|GetStarsRewardAmount))))))))))

(fn ConstructionScript)